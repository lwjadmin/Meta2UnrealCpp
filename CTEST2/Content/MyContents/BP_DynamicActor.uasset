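; BP_DynamicActor is an actor that builds its static mesh components dynamically instead of relying on pre-placed ones.
; The construction script adds a component showing BaseMesh and attaches it to SceneRoot.
; On BeginPlay, it asynchronously loads the soft-referenced SoftMesh, then adds a second component displaying it, offset upward and attached to the same root.
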(event EventBeginPlay
  (bind _object (Utilities|AsyncLoadAsset (Variables|Default|GetSoftMesh))
    (:Completed
      (bind _asstatic_mesh (Utilities|Casting|CastToStaticMesh _object))
      (bind _returnvalue (AddComponent|AddStaticMeshComponent false (Math|Transform|MakeTransform "0, 0,100.000000")))
      (Components|StaticMesh|SetStaticMesh _returnvalue _asstatic_mesh)
      (Transformation|AttachComponentToComponent _returnvalue (Variables|Default|GetSceneRoot) "None" "KeepRelative" "KeepRelative" "KeepRelative" true))))

(fn ConstructionScript
  (bind _returnvalue (AddComponent|AddStaticMeshComponent true))
  (Components|StaticMesh|SetStaticMesh _returnvalue (Variables|Default|GetBaseMesh))
  (Transformation|AttachComponentToComponent _returnvalue (Variables|Default|GetSceneRoot) "None" "KeepRelative" "KeepRelative" "KeepRelative" true))